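; Base character Blueprint shared by player and AI, where a player who dies takes control of their killer.
; OnMove treats its vector as movement input for the player character, or as an AIMoveTo destination that reports success or failure to the passed task.
; On player death, the killer's controller unpossesses it and the player controller possesses it with input enabled.
; Damage handling is only a debug print.
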(event `/Game/Player/BPI_Controllable.OnMove`
  (params (InputVector :type "Vector Structure") (Task :type "BTTask_BlueprintBase Object Reference"))
  (if (== self (`GameplayStatics.GetPlayerCharacter` 0))
    (`self.AddMovementInput` InputVector)
    (else
      (`|AIMoveTo` self InputVector null
        (:`OnSuccess`
          (`BTTask_BlueprintBase.FinishExecute` Task true))
        (:`OnFail`
          (`BTTask_BlueprintBase.FinishExecute` Task false))))))

(event `self.Health Component.OnDeath`
  (params (Killer :type "Character Object Reference"))
  (bind _returnvalue (`GameplayStatics.GetPlayerController` 0))
  (if (== self (`GameplayStatics.GetPlayerCharacter` 0))
    (`Controller.UnPossess` (`self.GetController` Killer))
    (`Controller.Possess` _returnvalue Killer)
    (`self.EnableInput` Killer _returnvalue)))

(event `self.Health Component.OnDamage`
  (`KismetSystemLibrary.PrintString` "Hello"))

(fn `UserConstructionScript`)