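; Player controller that turns Enhanced Input actions into messages for the possessed character.
; On possess it adds the player input mapping context and stores the pawn as the controlled character.
; Move input becomes a world-space vector from the character's forward and right vectors, and ability input is forwarded when it starts.
; The interact action is bound but does nothing.
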(event `self.ReceivePossess`
  (params (PossessedPawn :type "Pawn Object Reference"))
  (`EnhancedInputSubsystemInterface.AddMappingContext` (subsystem `EnhancedInputLocalPlayerSubsystem`) "/Game/Player/Input/IMC_PlayerInput.IMC_PlayerInput" 0 (struct))
  (set `self.ControlledCharacter` PossessedPawn))

(event `EnhancedInput|/Game/Player/Input/IA_Move`
  (params (ActionValue :type "Vector2D Structure") (ElapsedSeconds :type "Float (double-precision)") (TriggeredSeconds :type "Float (double-precision)") (InputAction :type "InputAction Object Reference" :default "/Game/Player/Input/IA_Move.IA_Move"))
  (bind _controlledcharacter (`self.ControlledCharacter`))
  (:`Triggered`
    (message `/Game/Player/BPI_Controllable.OnMove` (`self.ControlledCharacter`) (+ (* (`self.GetActorRightVector` _controlledcharacter) ActionValue_X) (* (`self.GetActorForwardVector` _controlledcharacter) ActionValue_Y)) null)))

(event `EnhancedInput|/Game/Player/Input/IA_Ability`
  (params (ActionValue :type Boolean) (ElapsedSeconds :type "Float (double-precision)") (TriggeredSeconds :type "Float (double-precision)") (InputAction :type "InputAction Object Reference" :default "/Game/Player/Input/IA_Ability.IA_Ability"))
  (:`Started`
    (message `/Game/Player/BPI_Controllable.OnAbility` (`self.ControlledCharacter`) null)))

(event `EnhancedInput|/Game/Player/Input/IA_Interact`
  (params (ActionValue :type Boolean) (ElapsedSeconds :type "Float (double-precision)") (TriggeredSeconds :type "Float (double-precision)") (InputAction :type "InputAction Object Reference" :default "/Game/Player/Input/IA_Interact.IA_Interact")))

(fn `UserConstructionScript`)